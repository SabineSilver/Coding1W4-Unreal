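; Spawn manager that runs endless enemy waves, starting shortly after BeginPlay.
; SpawnEnemies loops over every BP_SpawnPoint in the level and uses a weighted random roll to decide whether to spawn at each one.
; NewWaveCheck, meant to be called by dying enemies, counts remaining BP_Enemy actors and starts another wave after a delay when none remain.
; Debug prints trace each step.
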(event `self.ReceiveBeginPlay`
  (`KismetSystemLibrary.PrintString` "Spawn Manager exists")
  (`KismetSystemLibrary.Delay` 1.0)
  (`self.Spawn Enemies`))

(event `Spawn Enemies`
  (bind _outactors (`GameplayStatics.GetAllActorsOfClass` "/Game/Blueprints/BP_SpawnPoint.BP_SpawnPoint_C")) ; Get an array of all spawn points in the level
  (for _array_element _outactors
    (`KismetSystemLibrary.PrintString` (`KismetSystemLibrary.GetDisplayName` _array_element) true true (struct :`G` 0.229954 :`B` 0.63125 :`A` 1.0) 10.0)
    (if (`KismetMathLibrary.RandomBoolWithWeight` 0.8)
      (`|SpawnActorFromClass` "/Game/Blueprints/BP_Enemy.BP_Enemy_C" (`SceneComponent.K2_GetComponentToWorld` (`/Game/Blueprints/BP_SpawnPoint.DefaultSceneRoot` _array_element)) "Undefined" "MultiplyWithRoot" null null) ; spawn actor from class
    ))
  (`KismetSystemLibrary.PrintString` "Done with the For Each Loop for spawning enemies."))

(event `NewWaveCheck`
  (`KismetSystemLibrary.PrintString` "Was that the last enemy?")
  (bind _outactors (`GameplayStatics.GetAllActorsOfClass` "/Game/Blueprints/BP_Enemy.BP_Enemy_C"))
  (bind _returnvalue (`KismetArrayLibrary.Array_Length` _outactors))
  (`KismetSystemLibrary.PrintString` (`KismetStringLibrary.Concat_StrStr` "There are " (`KismetStringLibrary.Conv_IntToString` _returnvalue) " enemies in the level"))
  (if (> _returnvalue 0)
    (`KismetSystemLibrary.PrintString` "There are still more enemies!")
    (else
      (`KismetSystemLibrary.PrintString` "New wave incoming!" true true (struct :`R` 0.84 :`B` 0.032 :`A` 0.996))
      (`KismetSystemLibrary.Delay` 3.0)
      (`self.Spawn Enemies`))))

(fn `UserConstructionScript`)